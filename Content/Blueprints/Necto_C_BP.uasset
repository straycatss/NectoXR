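; Hand-tracking Blueprint that spawns a Bubble actor at the index fingertip when the left hand makes a pointing pose.
; BeginPlay binds to hand pose changes, and each update feeds the hand and pose name into PointToSpawnSphere.
; That function filters for the left hand's index point, picks the fingertip bone name by platform (Android differs), and spawns at its world location.
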(event Custom|HandPoseUpdated
  (params (Hand :type Oculus%20Hand%20Component%20Object%20Reference) (Pose :type Name))
  (CallFunction|PointtoSpawnSphere Hand Pose))

(event EventBeginPlay
  (|CallParentFunction)
  (EventDispatchers|BindEventtoHandPoseChanged (EventDispatchers|CreateEvent :!event Custom|HandPoseUpdated)))

(event Collision|EventActorBeginOverlap
  (params (OtherActor :type Actor%20Object%20Reference)))

(event EventTick
  (params (DeltaSeconds :type Float%20%28single-precision%29))
  (|CallParentFunction DeltaSeconds) ; This node is disabled and will not be called.\nDrag off pins to build functionality.
)

(fn ConstructionScript
  (|CallParentFunction))

(fn PointtoSpawnSphere
  (params (Hand :type Object%20Object%20Reference) (Gesture :type Name))
  (bind _hand_l (Variables|Default|GetHand_L))
  ;[1 1 1] Detect gesture
  (if (and (== Hand _hand_l) (Utilities|Name|Equal(Name) Gesture "index_point"))
    ;[1 1 1] Platform specific bone names
    (if (Utilities|Enum|Equal(Enum) (Game|GetPlatformName) "Android")
      (bind _output_get (LocalVariables|SetPlatformBoneName "Index_Tip"))
      (else
        (LocalVariables|SetPlatformBoneName "Index Tip")))
    ;[1 1 1] Spawn bubble
    (bind _returnvalue (Class|PoseableMeshComponent|GetBoneLocationbyName _hand_l _output_get "WorldSpace"))
    (Game|SpawnActorfromClass "/Game/Blueprints/Interactibles/Bubble.Bubble_C" (Math|Transform|MakeTransform _returnvalue) "Undefined" 0 0)))