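; An actor that shows a default text string in the world and keeps it facing the player's camera.
; BeginPlay sets the text, and SetCamera, which is not called within this Blueprint, caches player 0's PlayerCameraManager or prints an error.
; Once a camera is cached, Tick points the text's X axis at the camera location every frame, except on the server.
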(event Custom|SetCamera
  (bind _returnvalue (Game|GetPlayerController 0))
  (if (Utilities|IsValid _returnvalue)
    (Variables|Default|SetCameraParent (Variables|/Script/Engine.PlayerController|GetPlayerCameraManager _returnvalue))
    (Variables|Default|SetHasCamera true)
    (else
      (Development|PrintString "Could not find playercontroller"))))

(event EventBeginPlay
  (Rendering|Components|TextRender|SetText (Variables|Default|GetText) (Utilities|Text|ToText(String) (Variables|Default|GetDefaultText))))

(event EventTick
  (params (DeltaSeconds :type Float%20%28single-precision%29))
  (if (not (Networking|IsServer))
    (CallFunction|RotateTexttoCamera)))

(fn ConstructionScript)

(fn RotateTexttoCamera
  (if (Variables|Default|GetHasCamera)
    (Transformation|SetWorldRotation (Variables|Default|GetText) (Math|Rotator|MakeRotfromX (Math|Vector|Normalize (- (Camera|GetCameraLocation (Variables|Default|GetCameraParent)) (Transformation|GetWorldLocation (Variables|Default|GetText))))) false false)))