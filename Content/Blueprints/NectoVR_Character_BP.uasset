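; VR player character that lets the player grip and use objects with motion controllers or tracked hands.
; Tick switches input modes as hand tracking starts or stops, setting up hand physics capsules and toggling controller visibility.
; Grip buttons pass controller colliders, and finger pinches pass thumb and fingertip capsules, to StartGrip.
; StartGrip grips the closest grippable object, adding a secondary attachment when another controller already holds it.
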(event Custom|HandTrackingStart
  (params (Hands :type Set%20of%20Hand%20Component%20Object%20References))
  ;[1 1 1] Make hands active
  (CallFunction|MakeHandsActive Hands)
  (CallFunction|ToggleControllers false))

(event Custom|HandTrackingEnd
  ;[1 1 1] Make controllers active
  (CallFunction|ToggleControllers true)
  (Utilities|Array|Clear (Variables|Default|GetHandColliders)))

(event EventBeginPlay
  ;[1 1 1] Make controllers active
  (CallFunction|ToggleControllers true)
  (Utilities|Array|Clear (Variables|Default|GetHandColliders)))

(event EventTick
  (params (DeltaSeconds :type Float%20%28single-precision%29))
  (bind _returnvalue (Class|OculusInputFunctionLibrary|IsHandTrackingEnabled))
  ;[1 1 1] Switch between hands and controllers
  (if (and _returnvalue (not (Variables|Default|GetHandsDisplayed)))
    ;[1 1 1] Only get hands with valid skeletons
    (bind _activehands (CallFunction|GetValidHands))
    (if (> (Utilities|Set|Length _activehands) 0)
      (Variables|Default|SetHandsDisplayed _returnvalue)
      (CallFunction|HandTrackingStart _activehands))
    (elif (and (Variables|Default|GetHandsDisplayed) (not _returnvalue))
      ;[1 1 1] Switch to controllers
      (Variables|Default|SetHandsDisplayed _returnvalue)
      (CallFunction|HandTrackingEnd))))

(event Input|ActionEvents|InputActionVR_Grip_L
  (params (Key :type Key%20Structure :default "None"))
  (bind _leftmotioncontroller (Variables|Default|GetLeftMotionController))
  ;[1 1 1] Left hand grips
  (:Pressed
    ;;[1 1 1] Start controller grips (L)
    (CallFunction|StartGrip (Utilities|Set|MakeSet (Variables|Default|GetLeftMotionControllerCollision)) _leftmotioncontroller (Variables|Default|GetbDrawControllerColliders)))
  (:Released
    (CallFunction|ReleaseGrip _leftmotioncontroller)))

(event Input|ActionEvents|InputActionVR_Grip_R
  (params (Key :type Key%20Structure :default "None"))
  (bind _rightmotioncontroller (Variables|Default|GetRightMotionController))
  ;[1 1 1] Right hand grips
  (:Pressed
    ;;[1 1 1] Start controller grips (R)
    (CallFunction|StartGrip (Utilities|Set|MakeSet (Variables|Default|GetRightMotionControllerCollision)) _rightmotioncontroller (Variables|Default|GetbDrawControllerColliders)))
  (:Released
    (CallFunction|ReleaseGrip _rightmotioncontroller)))

(event Input|ActionEvents|InputActionMiddlePinch_L
  (params (Key :type Key%20Structure :default "None"))
  ;[1 1 1] Left hand grips
  (:Pressed
    ;;[1 1 1] Left hand pinch grips
    (bind _colliders (CallFunction|GetPinchColliders "Middle_3" (Variables|Default|GetLeftHand)))
    (CallFunction|StartGrip _colliders (Variables|Default|GetLeftMotionController) (Variables|Default|GetbDrawControllerColliders)))
  (:Released
    (CallFunction|ReleaseGrip (Variables|Default|GetLeftMotionController))))

(event Input|ActionEvents|InputActionRingPinch_L
  (params (Key :type Key%20Structure :default "None"))
  ;[1 1 1] Left hand grips
  (:Pressed
    ;;[1 1 1] Left hand pinch grips
    (bind _colliders (CallFunction|GetPinchColliders "Ring_3" (Variables|Default|GetLeftHand)))
    (CallFunction|StartGrip _colliders (Variables|Default|GetLeftMotionController) (Variables|Default|GetbDrawControllerColliders)))
  (:Released
    (CallFunction|ReleaseGrip (Variables|Default|GetLeftMotionController))))

(event Input|ActionEvents|InputActionPinkyPinch_L
  (params (Key :type Key%20Structure :default "None"))
  ;[1 1 1] Left hand grips
  (:Pressed
    ;;[1 1 1] Left hand pinch grips
    (bind _colliders (CallFunction|GetPinchColliders "Pinky_3" (Variables|Default|GetLeftHand)))
    (CallFunction|StartGrip _colliders (Variables|Default|GetLeftMotionController) (Variables|Default|GetbDrawControllerColliders)))
  (:Released
    (CallFunction|ReleaseGrip (Variables|Default|GetLeftMotionController))))

(event Input|ActionEvents|InputActionIndexPinch_R
  (params (Key :type Key%20Structure :default "None"))
  ;[1 1 1] Right hand grips
  (:Pressed
    ;;[1 1 1] Right hand pinch grips
    (bind _colliders (CallFunction|GetPinchColliders "Index_3" (Variables|Default|GetRightHand)))
    (CallFunction|StartGrip _colliders (Variables|Default|GetRightMotionController) (Variables|Default|GetbDrawControllerColliders)))
  (:Released
    (CallFunction|ReleaseGrip (Variables|Default|GetRightMotionController))))

(event Input|ActionEvents|InputActionMiddlePinch_R
  (params (Key :type Key%20Structure :default "None"))
  ;[1 1 1] Right hand grips
  (:Pressed
    ;;[1 1 1] Right hand pinch grips
    (bind _colliders (CallFunction|GetPinchColliders "Middle_3" (Variables|Default|GetRightHand)))
    (CallFunction|StartGrip _colliders (Variables|Default|GetRightMotionController) (Variables|Default|GetbDrawControllerColliders)))
  (:Released
    (CallFunction|ReleaseGrip (Variables|Default|GetRightMotionController))))

(event Input|ActionEvents|InputActionRingPinch_R
  (params (Key :type Key%20Structure :default "None"))
  ;[1 1 1] Right hand grips
  (:Pressed
    ;;[1 1 1] Right hand pinch grips
    (bind _colliders (CallFunction|GetPinchColliders "Ring_3" (Variables|Default|GetRightHand)))
    (CallFunction|StartGrip _colliders (Variables|Default|GetRightMotionController) (Variables|Default|GetbDrawControllerColliders)))
  (:Released
    (CallFunction|ReleaseGrip (Variables|Default|GetRightMotionController))))

(event Input|ActionEvents|InputActionPinkyPinch_R
  (params (Key :type Key%20Structure :default "None"))
  ;[1 1 1] Right hand grips
  (:Pressed
    ;;[1 1 1] Right hand pinch grips
    (bind _colliders (CallFunction|GetPinchColliders "Pinky_3" (Variables|Default|GetRightHand)))
    (CallFunction|StartGrip _colliders (Variables|Default|GetRightMotionController) (Variables|Default|GetbDrawControllerColliders)))
  (:Released
    (CallFunction|ReleaseGrip (Variables|Default|GetRightMotionController))))

(event Input|ActionEvents|InputActionVR_Trigger_R
  (params (Key :type Key%20Structure :default "None"))
  (:Pressed
    ;[1 1 1] Use the gripped actor (controller only)
    (CallFunction|StartUse (Variables|Default|GetRightMotionController))))

(event Input|ActionEvents|InputActionVR_Trigger_L
  (params (Key :type Key%20Structure :default "None"))
  (:Pressed
    ;[1 1 1] Use the gripped actor (controller only)
    (CallFunction|StartUse (Variables|Default|GetLeftMotionController))))

(event Input|ActionEvents|InputActionIndexPinch_L
  (params (Key :type Key%20Structure :default "None"))
  ;[1 1 1] Left hand grips
  (:Pressed
    ;;[1 1 1] Left hand pinch grips
    (bind _colliders (CallFunction|GetPinchColliders "Index_3" (Variables|Default|GetLeftHand)))
    (CallFunction|StartGrip _colliders (Variables|Default|GetLeftMotionController) (Variables|Default|GetbDrawControllerColliders)))
  (:Released
    (CallFunction|ReleaseGrip (Variables|Default|GetLeftMotionController))))

(fn ConstructionScript)

(fn GetGrippableOverlappingColliders
  (params (Colliders :type Set%20of%20Scene%20Component%20Object%20References))
  (bind _returnvalue (Math|Float|MakeLiteralFloat 5.0))
  (bind _colliderpositions (LocalVariables|GetColliderPositions))
  (bind _result (Utilities|Set|ToArray Colliders))
  ;[1 1 1] Only bother with multipler colliders if > 1
  (if (> (Utilities|Array|Length _result) 1)
    ;[1 1 1] Check for collision in a sphere from the bounds of all input colliders
    (for _array_element _result
      (Utilities|Array|Add _colliderpositions (Transformation|GetWorldLocation _array_element)))
    (bind _output_get (LocalVariables|SetCollisionCentroid (Math|Vector|GetVectorArrayAverage _colliderpositions)))
    (if (Utilities|Enum|Equal(Enum) (Game|GetPlatformName) "android")
      _
      (else
        (Rendering|Debug|DrawDebugSphere _output_get _returnvalue 12 "(R=1.000000,G=0.892180,B=0.000000,A=1.000000)" 5.0)))
    (bind _outactors (Collision|SphereOverlapActors _output_get _returnvalue (Utilities|Array|MakeArray "ObjectTypeQuery2" "ObjectTypeQuery1" "ObjectTypeQuery3" "ObjectTypeQuery4") 0))
    (LocalVariables|SetOverlappingActors _outactors)
    (else
      ;[1 1 1] Check for collision against a single actor
      (LocalVariables|SetCollisionCentroid (Transformation|GetActorLocation (Components|GetOwner (Utilities|Array|Get(acopy) _result (Utilities|Array|LastIndex _result)))))
      (LocalVariables|SetOverlappingActors (Collision|GetOverlappingActors (Components|GetOwner (Utilities|Array|Get(acopy) _result (Utilities|Array|LastIndex _result))) 0 :!class /Script/Engine.Actor))))
  (bind _closest (CallFunction|GetClosestGrippableActor (LocalVariables|GetOverlappingActors) (LocalVariables|GetCollisionCentroid)))
  (return _closest (LocalVariables|GetCollisionCentroid)))

(fn GetPinchColliders
  (params (Finger :type EBone%20Enum :default "Wrist_Root") (Hand :type Hand%20Component%20Object%20Reference))
  (bind _matchingcolliders (LocalVariables|GetMatchingColliders))
  ;[1 1 1] Add only the tips of the fingers/thumb so we can figure out the pinch location
  (for _array_element (Variables|/Script/OculusInput.OculusHandComponent|GetCollisionCapsules Hand)
    (if (or (Utilities|Enum|Equal(Enum) (.BoneId (Utilities|Struct|BreakOculusCapsuleCollider _array_element)) Finger) (== (.BoneId (Utilities|Struct|BreakOculusCapsuleCollider _array_element)) (Utilities|Enum|LiteralenumEBone "Thumb_3")))
      (Utilities|Set|Add _matchingcolliders (.Capsule (Utilities|Struct|BreakOculusCapsuleCollider _array_element)))
      (Development|PrintString (Utilities|String|Append "Adding capsule " (Class|OculusInputFunctionLibrary|GetBoneName (.BoneId (Utilities|Struct|BreakOculusCapsuleCollider _array_element)))))))
  (return _matchingcolliders))

(fn GetValidHands
  (bind _lefthand (Variables|Default|GetLeftHand))
  (bind _hands (LocalVariables|GetHands))
  (bind _righthand (Variables|Default|GetRightHand))
  (if (Variables|/Script/OculusInput.OculusHandComponent|GetbSkeletalMeshInitialized _lefthand)
    (Utilities|Set|Add _hands _lefthand))
  (if (Variables|/Script/OculusInput.OculusHandComponent|GetbSkeletalMeshInitialized _righthand)
    (Utilities|Set|Add _hands _righthand)
    (else
      (return _hands))))

(fn MakeHandsActive
  (params (Hands :type Set%20of%20Hand%20Component%20Object%20References))
  (Utilities|Array|Clear (Variables|Default|GetHandColliders))
  ;[1 1 1] Setup hand physics
  (bind _result (Utilities|Set|ToArray Hands))
  (for _array_element _result
    (Utilities|IsValid _array_element
      (:Is%20Valid
        (bind _returnvalue (Class|OculusInputFunctionLibrary|InitializeHandPhysics (Variables|/Script/OculusInput.OculusHandComponent|GetSkeletonType _array_element) _array_element 1e+02))
        ;[1 1 1] Make hand colliders overlap only
        (for _array_element_2 _returnvalue
          (Collision|SetCollisionProfileName (.Capsule (Utilities|Struct|BreakOculusCapsuleCollider _array_element_2)) "OverlapAllDynamic" true :!class /Script/Engine.PrimitiveComponent)
          (if (Variables|Default|GetbDrawControllerColliders)
            ;[0.1333 0.1019 0.0952] Debug hand collider visibility
            (Rendering|SetVisibility (.Capsule (Utilities|Struct|BreakOculusCapsuleCollider _array_element_2)) true true)
            (Development|SetHiddeninGame (.Capsule (Utilities|Struct|BreakOculusCapsuleCollider _array_element_2)) false false)))
        (Utilities|Array|AppendArray (Variables|Default|GetHandColliders) _returnvalue)))))

(fn StartGrip
  (params (Colliders :type Set%20of%20Scene%20Component%20Object%20References) (MotionController :type Grip%20Motion%20Controller%20Component%20Object%20Reference))
  (bind (_closestobject _collisionpoint) (CallFunction|GetGrippableOverlappingObjects Colliders 5.0 true))
  (Variables|Default|SetCollisionPoint _collisionpoint)
  (Utilities|IsValid _closestobject
    (:Is%20Valid
      (if (Utilities|DoesObjectImplementInterface _closestobject 0)
        ;[1 1 1] Find the original gripping controller
        (bind _asgrippable_actor (Utilities|Casting|CastToGrippableActor _closestobject)
          (:then
            (bind _output_get (LocalVariables|SetGrippedObject _asgrippable_actor)))
          (:CastFailed
            (bind _asgrippable_static_mesh_component (Utilities|Casting|CastToGrippableStaticMeshComponent _closestobject))
            (LocalVariables|SetGrippedObject _asgrippable_static_mesh_component)))
        (bind (_holdingcontrollers _bisheld) (Class|VRGripInterface|IsHeld(Message) _output_get))
        (if _bisheld
          (for _array_element _holdingcontrollers
            (if (!= (.HoldingController (Utilities|Struct|BreakBPGripPair _array_element)) MotionController)
              (LocalVariables|SetOtherGripController (.HoldingController (Utilities|Struct|BreakBPGripPair _array_element)))))
          (Utilities|IsValid (LocalVariables|GetOtherGripController)
            (:Is%20Valid
              ;[1 1 1] Secondary grip
              (Class|GripMotionControllerComponent|AddSecondaryAttachmentPoint (LocalVariables|GetOtherGripController) _closestobject MotionController (Transformation|GetWorldTransform MotionController) false 0.0 false "None"))
            (:Is%20Not%20Valid
              ;[1 1 1] First grip
              (Class|GripMotionControllerComponent|GripObjectbyInterface MotionController _closestobject (Transformation|GetWorldTransform (Variables|Transformation|GetRootComponent)) false "None" "None" false :!label _label)))
          (else
            (goto _label)))))))

(fn ToggleControllers
  (params (Visible :type Boolean))
  (bind _returnvalue (not Visible))
  (Rendering|SetVisibility (Variables|Default|GetLeftMotionController) Visible false)
  (Rendering|SetVisibility (Variables|Default|GetRightMotionController) Visible false)
  (if (Variables|Default|GetbDrawControllerColliders)
    (Rendering|SetVisibility (Variables|Default|GetLeftMotionControllerCollision) Visible false)
    (Rendering|SetVisibility (Variables|Default|GetRightMotionControllerCollision) Visible false))
  (for _array_element (Variables|Default|GetHandColliders)
    (if _returnvalue
      (bind _output_get (LocalVariables|SetHandCollisionProfile "BlockAll"))
      (else
        (LocalVariables|SetHandCollisionProfile "NoCollision")))
    (Collision|SetCollisionProfileName (.capsule _array_element) _output_get true :!class /Script/Engine.PrimitiveComponent)
    (if (Variables|Default|GetbDrawControllerColliders)
      (Rendering|SetVisibility (.capsule _array_element) _returnvalue false))))