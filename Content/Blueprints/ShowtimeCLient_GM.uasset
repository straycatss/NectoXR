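; Game mode for the Showtime client that advertises an online session on dedicated servers and assigns player spawn points.
; On BeginPlay, a dedicated server runs an AdvancedSession call and logs when it succeeds.
; The construction script caches all PlayerStarts, and ChoosePlayerStart cycles through them round-robin with an incrementing index, printing each pick.
; ReadyToStartMatch always returns true, so the match never waits to start.
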(event EventBeginPlay
  (bind _returnvalue (Networking|IsDedicatedServer))
  (if _returnvalue
    (|AdvancedSession 0 0 100 0 false true _returnvalue true true false false false true
      (:OnSuccess
        (Development|PrintString "Advertising session" false)))))

(fn ConstructionScript
  ;[1 1 1] Save playerstarts for cycling through
  (bind _outactors (Actor|GetAllActorsOfClass "/Script/Engine.PlayerStart"))
  (Variables|Default|SetPlayerStarts _outactors))

(fn ChoosePlayerStart
  (params (Player :type Controller%20Object%20Reference))
  ;[1 1 1] Cycle through all available playerstarts cached at the start
  (bind _result (Math|Integer|IncrementInt (Variables|Default|GetLastPlayerStartIndex))
    (:%20%20
      (Development|PrintString (Utilities|String|Append "Picking playerstart" (Utilities|GetDisplayName (Utilities|Array|Get(acopy) (Variables|Default|GetPlayerStarts) (Math|Integer|%(Integer) _result (Utilities|Array|Length (Variables|Default|GetPlayerStarts)))))))
      (return (Utilities|Array|Get(acopy) (Variables|Default|GetPlayerStarts) (Math|Integer|%(Integer) _result (Utilities|Array|Length (Variables|Default|GetPlayerStarts))))))))

(fn ReadytoStartMatch
  (return true))