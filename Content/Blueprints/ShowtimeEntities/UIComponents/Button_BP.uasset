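; Button_BP is a VR button entity for the Showtime system that sends an integer value through a plug when its state turns on.
; Construction binds the VRButton state event and, with authority, gets the ShowtimePlug from a child Plug_A_BP actor.
; It then registers its component under the BrowserGamemode client's root performer, with the plug as that component's child.
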(event Custom|OnButtonStateChanged
  (params (ButtonState :type Boolean) (InteractingActor :type Actor%20Object%20Reference) (InteractingComponent :type Primitive%20Component%20Object%20Reference))
  (if ButtonState
    (Class|ShowtimePlug|SetIntValues (Variables|Default|GetPlug) (Utilities|Array|MakeArray (Variables|Default|GetSendVal)))))

(event EventBeginPlay)

(event Collision|EventActorBeginOverlap
  (params (OtherActor :type Actor%20Object%20Reference)))

(event EventTick
  (params (DeltaSeconds :type Float%20%28single-precision%29)))

(fn ConstructionScript
  (bind _component_ac_bp (Variables|Default|GetComponent_AC_BP))
  ;[1 1 1] Bind events
  (EventDispatchers|BindEventtoOnButtonStateChanged (Variables|Default|GetVRButton) (EventDispatchers|CreateEvent :!event Custom|OnButtonStateChanged))
  ;[1 1 1] Get plug entities
  (Networking|SwitchHasAuthority
    (:Authority
      (bind _asplug_a_bp (Utilities|Casting|CastToPlug_A_BP (Variables|/Script/Engine.ChildActorComponent|GetChildActor (Variables|Default|GetChildPlug_AC))))
      (Variables|Default|SetPlug (Actor|GetComponentbyClass _asplug_a_bp "/Script/ShowtimeRuntime.ShowtimePlug"))
      ;[1 1 1] Add button entities to client
      (bind _asbrowser_gamemode (Utilities|Casting|CastToBrowserGamemode (Game|GetGameMode)))
      (Class|ShowtimeEntity|AddChild (Class|ShowtimeClient|GetRootPerformer (Variables|/Game/Blueprints/BrowserGamemode.BrowserGamemode_C|GetShowtimeClient _asbrowser_gamemode)) _component_ac_bp)
      (Class|ShowtimeEntity|AddChild _component_ac_bp (Actor|GetComponentbyClass _asplug_a_bp "/Script/ShowtimeRuntime.ShowtimePlug")))))