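; Showtime client Blueprint that discovers graph servers and manages the connection from BeginPlay to EndPlay.
; While unconnected, each discovered server spawns a ServerBeacon_BP at "lobby_start", is stored in Servers, and gets auto-joined.
; Arriving component entities have their owners scattered in a random cone to avoid flying apart; performer children are printed after graph sync.
; The network server instance suffixes its client name and removes lost servers.
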(event Custom|On%20Graph%20Synchronised
  (params (Client :type Showtime%20Client%20Object%20Reference) (ServerAddress :type Server%20Address%20Structure))
  ;[1 1 1] List received performers after we've finished synchronising
  (for _array_element (Class|ShowtimeClient|GetPerformers Client)
    (for _array_element_2 (Class|ShowtimeEntity|GetChildren _array_element true)
      (Development|PrintString (Utilities|String|Append "Found entity " (Variables|/Script/ShowtimeRuntime.ShowtimeEntity|GetEntityPath _array_element_2))))))

(event Custom|On%20Server%20Discovered
  (params (Client :type Showtime%20Client%20Object%20Reference) (ServerAddress :type Server%20Address%20Structure))
  ;[1 1 1] Server discovery
  (Development|PrintString (Utilities|String|Append "Received server beacon " (.name ServerAddress)))
  (if (not (Class|ShowtimeClient|IsConnected Client))
    ;;[1 1 1] Spawn beacon
    (bind _returnvalue (Game|SpawnActorfromClass "/Game/Blueprints/ServerBeacon_BP.ServerBeacon_BP_C" (Transformation|GetActorTransform (Class|GameModeBase|FindPlayerStart (Game|GetGameMode) 0 "lobby_start")) "Undefined" 0 (.name ServerAddress) 0))
    (Default|SetOwningClient _returnvalue Client)
    (Utilities|Map|Add (Variables|Default|GetServers) (.name ServerAddress) _returnvalue)
    ;[1 1 1] Autojoin first found beacon
    (if (not (Class|ShowtimeClient|IsConnected Client))
      (Class|ShowtimeClient|JoinServerbyName Client (.name ServerAddress)))))

(event Custom|On%20Server%20Lost
  (params (Client :type Showtime%20Client%20Object%20Reference) (ServerAddress :type Server%20Address%20Structure))
  ;[1 1 1] Server discovery
  (if (Networking|IsServer)
    (Utilities|Map|Remove (Variables|Default|Getservers) (.name ServerAddress))))

(event Custom|On%20Connected%20To%20Server
  (params (Client :type Showtime%20Client%20Object%20Reference) (ServerAddress :type Server%20Address%20Structure))
  ;[1 1 1] Print connected
  (Development|PrintString (Utilities|String|Append "Connected to graph server " (.name ServerAddress))))

(event Custom|On%20Entity%20Arriving
  (params (entity :type Showtime%20Entity%20Object%20Reference))
  ;[1 1 1] Random starting location to avoid components flying into space
  (bind _asshowtime_component (Utilities|Casting|CastToShowtimeComponent entity))
  (Transformation|SetActorLocation (Components|GetOwner _asshowtime_component) (+ (* (Math|Random|RandomUnitVectorinConeinDegrees "0,1.000000,1.000000" 45.0) (Math|Random|RandomFloatinRange 0.0 1e+02)) "0, 0,100.000000") false false)
  (Development|PrintString (Utilities|String|Append "Received entity " (Variables|/Script/ShowtimeRuntime.ShowtimeEntity|GetEntityPath _asshowtime_component))))

(event EventBeginPlay
  ;[1 1 1] Assign events and init client
  (EventDispatchers|AssignOnServerDiscovered (EventDispatchers|CreateEvent :!event Custom|On%20Server%20Discovered))
  (EventDispatchers|BindEventtoOnServerLost (EventDispatchers|CreateEvent :!event Custom|On%20Server%20Lost))
  (EventDispatchers|BindEventtoOnConnectedtoServer (EventDispatchers|CreateEvent :!event Custom|On%20Connected%20To%20Server))
  (EventDispatchers|BindEventtoOnEntityArriving (EventDispatchers|CreateEvent :!event Custom|On%20Entity%20Arriving))
  (EventDispatchers|BindEventtoOnGraphSynchronised (EventDispatchers|CreateEvent :!event Custom|On%20Graph%20Synchronised))
  (CallFunction|InitClient))

(event EventEndPlay
  (params (EndPlayReason :type EEndPlayReason%20Enum :default "Destroyed"))
  (Class|ShowtimeClient|LeaveServer))

(fn InitClient
  ;[1 1 1] Init Showtime client
  (if (Networking|IsServer)
    (Variables|Default|SetClientName (Utilities|String|Append (Variables|Default|GetClientName) "_serv")))
  (Class|ShowtimeClient|Init)
  (return))