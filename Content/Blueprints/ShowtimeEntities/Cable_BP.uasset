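; Cable actor that draws a spline-mesh cable behind a spawned jack and connects two plugs.
; While drawing, Tick appends a spline point at the jack's position every frame, adding a mesh segment with its own dynamic material.
; ConnectCable sorts the plugs into input and output and forwards them to the origin plug's OwningClient.
; Ghost status selects a segment colour from a map, though the material parameter name is None.
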(event EventTick
  (params (DeltaSeconds :type Float%20%28single-precision%29))
  (bind _drawingjack (Variables|Default|GetDrawingJack))
  (bind _currentpoint (Variables|Default|GetCurrentPoint))
  (bind _spline (Variables|Default|GetSpline))
  (bind (_location _tangent) (Spline|GetLocationandTangentatSplinePoint _spline _currentpoint "Local"))
  (bind _returnvalue (- _currentpoint 1))
  (bind (_location_2 _tangent_2) (Spline|GetLocationandTangentatSplinePoint _spline _returnvalue "Local"))
  ;[1 1 1] Determine if we are actively drawing this cable
  (Networking|SwitchHasAuthority
    (:Authority
      _)
    (:Remote
      _))
  (if (and (Variables|Default|GetbIsDrawing) (Utilities|IsValid _drawingjack))
    ;[1 1 1] Add a new point to the drawn spline
    (bind _result (Math|Integer|IncrementInt (Variables|Default|GetCurrentPoint))
      (:%20%20
        (Class|SplineComponent|AddPoint (Variables|Default|GetSpline) (Utilities|Struct|MakeSplinePoint (Math|Conversions|ToFloat(Integer) _result) (- (Transformation|GetActorLocation _drawingjack) (Transformation|GetActorLocation))) true)
        ;[1 1 1] Add a new spline mesh component
        (if (> _currentpoint 1)
          (bind _returnvalue_2 (AddComponent|AddSplineMeshComponent false))
          (SplineMesh|SetStartandEnd _returnvalue_2 _location_2 _tangent_2 _location _tangent true :!class /Script/Engine.SplineMeshComponent)
          ;;[1 1 1] Create dynamic materials for spline segments
          (bind _returnvalue_3 (Rendering|Material|CreateDynamicMaterialInstance _returnvalue_2 0 (Rendering|Material|GetMaterial _returnvalue_2 0) "None" :!class /Script/Engine.PrimitiveComponent))
          (Utilities|Array|Add (Variables|Default|GetCableDynMats) _returnvalue_3))))))

(fn ConstructionScript
  (bind _spline (Variables|Default|GetSpline))
  (Spline|ClearSplinePoints _spline true)
  (Spline|AddSplinePoint _spline (Math|Vector|MakeVector 0.0 0.0 0.0) "Local" true)
  (CallFunction|SetCableGhostStatus "NewEnumerator2"))

(fn StartDrawing
  (params (OriginPlug :type Showtime%20Plug%20Object%20Reference))
  (bind _output_get (Variables|Default|SetOriginPlug OriginPlug))
  (Variables|Default|SetbIsDrawing true)
  (bind _returnvalue (Game|SpawnActorfromClass "/Game/Blueprints/Interaction/CableJack_A_BP.CableJack_A_BP_C" (Math|Transform|MakeTransform (Transformation|GetActorLocation (Components|GetOwner _output_get))) "Undefined" 0 self 0))
  (bind _output_get_2 (Variables|Default|SetDrawingJack _returnvalue))
  (return _output_get_2))

(fn ConnectCable
  (params (DroppedOnPlug :type Showtime%20Plug%20Object%20Reference) (OriginPlug :type Showtime%20Plug%20Object%20Reference))
  (bind (_inputplug _outputplug) (CallFunction|SortPlugs DroppedOnPlug OriginPlug))
  (Class|ShowtimeClient|ConnectCable (Variables|/Script/ShowtimeRuntime.ShowtimeEntity|GetOwningClient OriginPlug) _inputplug _outputplug))

(fn SetCableGhostStatus
  (params (Status :type CableGhostStatus%20Enum :default "NewEnumerator2"))
  (bind _output_get (Variables|Default|SetCableGhosting Status))
  (for _array_element (Variables|Default|GetCableDynMats)
    (Rendering|Material|SetVectorParameterValue _array_element "None" (Math|Conversions|ToLinearColor(Color) (.Value (Utilities|Map|Find (Variables|Default|GetCableColours) _output_get))) :!class /Script/Engine.MaterialInstanceDynamic)))