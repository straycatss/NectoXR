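; Networked plug actor for a Showtime entity that a player grips to pull out a new cable.
; On grip, the server spawns a Cable_BP, starts drawing it from the plug component and hands the returned jack to the gripping controller.
; When the plug component initialises, the server sets replicated label and direction.
; RepNotifies update the text and the "Activated" parameter of a dynamic material created on remotes, distinguishing inputs from outputs.
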(event Custom|OnInitialised
  (bind _plug_ac_bp (Variables|Default|GetPlug_AC_BP))
  (Networking|SwitchHasAuthority
    (:Authority
      (Variables|Default|SetPlugLabel (Utilities|Text|ToText(String) (Variables|/Script/ShowtimeRuntime.ShowtimeEntity|GetEntityPath _plug_ac_bp)))
      (Variables|Default|SetPlugDirection (Class|ShowtimePlug|Direction _plug_ac_bp)))))

(event EventOnGripRelease
  (params (ReleasingController :type Grip%20Motion%20Controller%20Component%20Object%20Reference) (GripInformation :type BP%20Actor%20Grip%20Information%20Structure%20%28by%20ref%29) (bWasSocketed :type Boolean))
  (Networking|SwitchHasAuthority))

(event EventOnGrip
  (params (GrippingController :type Grip%20Motion%20Controller%20Component%20Object%20Reference) (GripInformation :type BP%20Actor%20Grip%20Information%20Structure%20%28by%20ref%29))
  (Networking|SwitchHasAuthority
    (:Authority
      ;[1 1 1] Spawn cable at plug
      (bind _returnvalue (Game|SpawnActorfromClass "/Game/Blueprints/ShowtimeEntities/Cable_BP.Cable_BP_C" (Math|Conversions|ToTransform(Vector) (Transformation|GetActorLocation)) "Undefined" (Components|GetOwner GrippingController) 0))
      ;[1 1 1] Pass grip event to cable jack
      (bind _drawingjack (Default|StartDrawing _returnvalue (Variables|Default|GetPlug_AC_BP)))
      (Class|GripMotionControllerComponent|GripObjectbyInterface GrippingController _drawingjack (Transformation|GetWorldTransform (Variables|/Script/Engine.Actor|GetRootComponent _drawingjack)) false "None" "None" false))))

(fn ConstructionScript
  (Networking|SwitchHasAuthority
    (:Authority
      _)
    (:Remote
      (bind _returnvalue (Rendering|Material|CreateDynamicMaterialInstance (Rendering|Material|GetMaterial (Variables|Default|GetStaticMeshComponent) 0) "None" :!class /Script/Engine.KismetMaterialLibrary))
      (Variables|Default|SetDynMat _returnvalue)))
  (EventDispatchers|BindEventtoOnInitialised (Variables|Default|GetPlug_AC_BP) (EventDispatchers|CreateEvent :!event Custom|OnInitialised)))

(fn OnRepPlugDirection
  (bind _dynmat (Variables|Default|GetDynMat))
  (switch Utilities|FlowControl|Switch|SwitchonUShowtimePlugDirection (Variables|Default|GetPlugDirection)
    (:Direction_In
      (Rendering|Material|SetScalarParameterValue _dynmat "Activated" 1.0 :!class /Script/Engine.MaterialInstanceDynamic))
    (:Direction_Out
      (Rendering|Material|SetScalarParameterValue _dynmat "Activated" 0.0 :!class /Script/Engine.MaterialInstanceDynamic))))

(fn OnRepPlugLabel
  (Rendering|Components|TextRender|SetText (Variables|Default|GetTextRender) (Variables|Default|GetPlugLabel)))