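; Grippable cable jack actor that serves as the loose end of a cable and completes the connection when dropped on a plug.
; On grip release, the authority finds the overlapping Plug_A_BP closest to the releasing controller and has OwningCable connect it to its origin plug.
; With no plug found, the cable is destroyed; either way drawing ends and the jack destroys itself.
; Grip and grip-tick handlers are empty stubs.
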(event EventOnGrip
  (params (GrippingController :type Grip%20Motion%20Controller%20Component%20Object%20Reference) (GripInformation :type BP%20Actor%20Grip%20Information%20Structure%20%28by%20ref%29))
  (if (Variables|/Game/Blueprints/ShowtimeEntities/Cable_BP.Cable_BP_C|GetbIsDrawing (Variables|Default|GetOwningCable))
    _))

(event EventOnGripRelease
  (params (ReleasingController :type Grip%20Motion%20Controller%20Component%20Object%20Reference) (GripInformation :type BP%20Actor%20Grip%20Information%20Structure%20%28by%20ref%29) (bWasSocketed :type Boolean))
  (bind _owningcable (Variables|Default|GetOwningCable))
  (Networking|SwitchHasAuthority
    (:Authority
      (bind _closest (CallFunction|GetClosestGrippableActor (Collision|GetOverlappingActors (Variables|Default|GetStaticMeshComponent) "/Game/Blueprints/ShowtimeEntities/Plug_A_BP.Plug_A_BP_C" :!class /Script/Engine.PrimitiveComponent) (Transformation|GetWorldLocation ReleasingController)))
      (bind _asplug_a_bp (Utilities|Casting|CastToPlug_A_BP _closest)
        (:then
          (Default|ConnectCable _owningcable (Actor|GetComponentbyClass _asplug_a_bp "/Script/ShowtimeRuntime.ShowtimePlug") (Variables|/Game/Blueprints/ShowtimeEntities/Cable_BP.Cable_BP_C|GetOriginPlug _owningcable)))
        (:CastFailed
          (Actor|DestroyActor (Variables|Default|GetOwningCable))))
      (Variables|/Game/Blueprints/ShowtimeEntities/Cable_BP.Cable_BP_C|SetbIsDrawing _owningcable false)
      (Actor|DestroyActor))))

(event EventTickGrip
  (params (GrippingController :type Grip%20Motion%20Controller%20Component%20Object%20Reference) (GripInformation :type BP%20Actor%20Grip%20Information%20Structure%20%28by%20ref%29) (DeltaTime :type Float%20%28single-precision%29))
  (if (Variables|/Game/Blueprints/ShowtimeEntities/Cable_BP.Cable_BP_C|GetbIsDrawing (Variables|Default|GetOwningCable))
    (Utilities|IsValid GrippingController)))

(fn ConstructionScript)