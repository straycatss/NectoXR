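; An actor component that attaches a plug's owning actor to its own owner at a random point around it.
; AttachPlug snaps the plug actor to the owner, parents it, copies the owner's scale as relative scale, then offsets it 50 units along a random unit vector.
; Its relative rotation is then set from the world-space direction back toward the owner's origin.
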(event EventAttachPlug
  (params (plug :type Showtime%20Plug%20Object%20Reference))
  (bind _returnvalue (Components|GetOwner))
  (bind _returnvalue_2 (Components|GetOwner plug))
  (Transformation|SetActorLocation _returnvalue_2 (Transformation|GetActorLocation _returnvalue) false false)
  (Transformation|AttachActorToActor _returnvalue_2 _returnvalue "None" "KeepWorld" "SnapToTarget" "KeepRelative" true)
  (Transformation|SetActorRelativeScale3D _returnvalue_2 (Transformation|GetActorScale3D _returnvalue))
  (Transformation|SetActorRelativeLocation _returnvalue_2 (* (Math|Random|RandomUnitVector) 5e+01))
  (Transformation|SetActorRelativeRotation _returnvalue_2 (Math|Conversions|RotationFromXVector (- (Transformation|GetActorLocation _returnvalue) (Transformation|GetActorLocation _returnvalue_2)))))