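; A label actor that keeps its text turned relative to the local VR player, showing DefaultLabelText from BeginPlay.
; The SetCamera event casts player 0's pawn to NectoVR_Character_BP and caches the owner of its VRReplicatedCamera.
; Once that is set, each Tick points the label's X axis away from that owner's root component, which serves as the view position instead of the camera itself.
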(event Custom|SetCamera
  (bind _asnecto_vr_character_bp (Utilities|Casting|CastToNectoVR_Character_BP (Pawn|GetControlledPawn (Game|GetPlayerController 0))))
  (Variables|Default|SetCameraParent (Components|GetOwner (Variables|/Script/VRExpansionPlugin.VRBaseCharacter|GetVRReplicatedCamera _asnecto_vr_character_bp)))
  (Variables|Default|SetHasCamera true))

(event EventBeginPlay
  (Variables|Default|Setlabel (Variables|Default|Getlabel))
  (Rendering|Components|TextRender|SetText (Variables|Default|Getlabel) (Utilities|Text|ToText(String) (Variables|Default|GetDefaultLabelText))))

(event EventTick
  (params (DeltaSeconds :type Float%20%28single-precision%29))
  (CallFunction|RotateLabeltoCamera))

(fn ConstructionScript)

(fn RotateLabeltoCamera
  (if (Variables|Default|GetHasCamera)
    (Transformation|SetWorldRotation (Variables|Default|Getlabel) (Math|Rotator|MakeRotfromX (Math|Vector|Normalize (- (Transformation|GetWorldLocation (Variables|Default|Getlabel)) (Transformation|GetWorldLocation (Variables|/Script/Engine.Actor|GetRootComponent (Variables|Default|GetCameraParent)))))) false false)))