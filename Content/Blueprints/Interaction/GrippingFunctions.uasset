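; Blueprint function library for VR hand interaction, handling grip, release and use of objects implementing VRGripInterface.
; StartGrip finds a nearby grippable component or actor by distance, using owner overlaps for one collider or a sphere overlap at the centroid of several.
; An object already held by another controller gets a secondary attachment; otherwise it is gripped with the gripper component as pivot.
; Helpers find the closest grippable actor and average two component transforms.
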(fn GetClosestGrippableActor
  (params (OverlappingActors :type Array%20of%20Actor%20Object%20References) (CollisionPoint :type Vector))
  ;[1 1 1] Find closest grippable actor
  (for _array_element OverlappingActors
    (if (Utilities|DoesObjectImplementInterface _array_element "/Script/VRExpansionPlugin.VRGripInterface")
      (Utilities|IsValid (LocalVariables|GetClosestActor)
        (:Is%20Valid
          (if (< (Math|Vector|VectorLength (- (Transformation|GetActorLocation _array_element) CollisionPoint)) (LocalVariables|GetClosestDistance))
            (LocalVariables|SetClosestDistance (Math|Vector|VectorLength (- (Transformation|GetActorLocation _array_element) CollisionPoint)) :!label _label)
            (bind _output_get (LocalVariables|SetClosestActor _array_element))))
        (:Is%20Not%20Valid
          (goto _label)))))
  (return _output_get))

(fn GetGrippableOverlappingObjects
  (params (Colliders :type Set%20of%20Scene%20Component%20Object%20References) (CollisionRadius :type Float%20%28single-precision%29) (DrawCollision :type Boolean))
  (bind _colliderpositions (LocalVariables|GetColliderPositions))
  (LocalVariables|SetCollisionRad CollisionRadius)
  (LocalVariables|SetbShouldDrawCollision DrawCollision)
  ;[1 1 1] Only bother with multipler colliders if > 1
  (bind _result (Utilities|Set|ToArray Colliders))
  (if (> (Utilities|Array|Length _result) 1)
    ;[1 1 1] Check for collision in a sphere from the bounds of all input colliders
    ;;[1 1 1] Average position of colliders
    (for _array_element _result
      (Utilities|Array|Add _colliderpositions (Transformation|GetWorldLocation _array_element)))
    (bind _output_get (LocalVariables|SetCollisionCentroid (Math|Vector|GetVectorArrayAverage _colliderpositions)))
    (if (LocalVariables|GetbShouldDrawCollision)
      (Rendering|Debug|DrawDebugSphere 0 _output_get (LocalVariables|GetCollisionRad) 12 "(R=1.000000,G=0.892180,B=0.000000,A=1.000000)" 5.0))
    (bind _outactors (Collision|SphereOverlapActors 0 _output_get (LocalVariables|GetCollisionRad) (Utilities|Array|MakeArray "ObjectTypeQuery2" "ObjectTypeQuery1" "ObjectTypeQuery3" "ObjectTypeQuery4")))
    (LocalVariables|SetOverlappingActors _outactors)
    (else
      ;[1 1 1] Check for collision against a single actor
      (LocalVariables|SetCollisionCentroid (Transformation|GetActorLocation (Components|GetOwner (Utilities|Array|Get(acopy) _result (Utilities|Array|LastIndex _result)))))
      (LocalVariables|SetOverlappingActors (Collision|GetOverlappingActors (Components|GetOwner (Utilities|Array|Get(acopy) _result (Utilities|Array|LastIndex _result))) 0 :!class /Script/Engine.Actor))))
  (for _array_element_2 (LocalVariables|GetOverlappingActors)
    ;[1 1 1] Grippable component in overlapping actor?
    (if (> (Utilities|Array|Length (Class|Actor|GetComponentsbyInterface _array_element_2 "/Script/VRExpansionPlugin.VRGripInterface")) 0)
      (for _array_element_3 (Class|Actor|GetComponentsbyInterface _array_element_2 "/Script/VRExpansionPlugin.VRGripInterface")
        ;;[1 1 1] Find closest grippable component
        (Utilities|IsValid (LocalVariables|GetClosestObj)
          (:Is%20Valid
            (if (< (Math|Vector|VectorLength (- (Transformation|GetActorLocation (Components|GetOwner _array_element_3)) (LocalVariables|GetCollisionCentroid))) (LocalVariables|GetClosestDistance))
              (LocalVariables|SetClosestDistance (Math|Vector|VectorLength (- (Transformation|GetActorLocation (Components|GetOwner _array_element_3)) (LocalVariables|GetCollisionCentroid))) :!label _label)
              (bind _asprimitive_component (Utilities|Casting|CastToPrimitiveComponent _array_element_3))
              (LocalVariables|SetClosestObj _asprimitive_component)))
          (:Is%20Not%20Valid
            (goto _label))))
      (return (LocalVariables|GetClosestObj) (LocalVariables|GetCollisionCentroid))
      (else
        ;[1 1 1] Find closest grippable actor
        (if (Utilities|DoesObjectImplementInterface _array_element_2 "/Script/VRExpansionPlugin.VRGripInterface")
          (Utilities|IsValid (LocalVariables|GetClosestObj)
            (:Is%20Valid
              (if (< (Math|Vector|VectorLength (- (Transformation|GetActorLocation _array_element_2) (LocalVariables|GetCollisionCentroid))) (LocalVariables|GetClosestDistance))
                (LocalVariables|SetClosestDistance (Math|Vector|VectorLength (- (Transformation|GetActorLocation _array_element_2) (LocalVariables|GetCollisionCentroid))) :!label _label_2)
                (LocalVariables|SetClosestObj _array_element_2)))
            (:Is%20Not%20Valid
              (goto _label_2)))))))
  (return (LocalVariables|GetClosestObj) (LocalVariables|GetCollisionCentroid)))

(fn StartGrip
  (params (GripperComponent :type Scene%20Component%20Object%20Reference%20%28by%20ref%29) (MotionController :type Grip%20Motion%20Controller%20Component%20Object%20Reference) (DrawCollision :type Boolean))
  (bind _output_get (LocalVariables|SetController MotionController))
  (LocalVariables|SetGripPoint GripperComponent)
  ;[1 1 1] Get closest valid grippable object
  (bind _closestobject (CallFunction|GetGrippableOverlappingObjects (Utilities|Set|MakeSet GripperComponent) 5.0 DrawCollision _output_get))
  (Utilities|IsValid _closestobject
    (:Is%20Valid
      (bind _output_get_2 (LocalVariables|SetGrippedObject _closestobject))
      (if (Utilities|DoesObjectImplementInterface _output_get_2 "/Script/VRExpansionPlugin.VRGripInterface")
        ;[1 1 1] Find the original gripping controller
        (bind _asvrgrip_interface (Utilities|Casting|CastToVRGripInterface _output_get_2))
        (bind (_holdingcontrollers _bisheld) (Class|VRGripInterface|IsHeld(Message) (Utilities|ToObject(Interface) _asvrgrip_interface)))
        (if _bisheld
          (for _array_element _holdingcontrollers
            (if (!= (.HoldingController (Utilities|Struct|BreakBPGripPair _array_element)) (LocalVariables|GetController))
              (LocalVariables|SetOtherGripController (.HoldingController (Utilities|Struct|BreakBPGripPair _array_element)))))
          (Utilities|IsValid (LocalVariables|GetOtherGripController)
            (:Is%20Valid
              ;[1 1 1] Secondary grip
              (Class|GripMotionControllerComponent|AddSecondaryAttachmentPoint (LocalVariables|GetOtherGripController) (LocalVariables|GetGrippedObject) (LocalVariables|GetController) (Transformation|GetWorldTransform (LocalVariables|GetController)) false 0.0 false "None"))
            (:Is%20Not%20Valid
              ;[1 1 1] First grip
              (bind _asactor (Utilities|Casting|CastToActor (LocalVariables|GetGrippedObject) :!label _label)
                (:then
                  (LocalVariables|SetGrippedObjectTransform (Transformation|GetWorldTransform (Variables|/Script/Engine.Actor|GetRootComponent _asactor))))
                (:CastFailed
                  (bind _asprimitive_component (Utilities|Casting|CastToPrimitiveComponent (LocalVariables|GetGrippedObject)))
                  (LocalVariables|SetGrippedObjectTransform (Transformation|GetWorldTransform _asprimitive_component))))
              (Class|GripMotionControllerComponent|SetCustomPivotComponent (LocalVariables|GetController) (LocalVariables|GetGripPoint))
              (Class|GripMotionControllerComponent|GripObjectbyInterface (LocalVariables|GetController) (LocalVariables|GetGrippedObject) (LocalVariables|GetGrippedObjectTransform) false "None" "None" false)))
          (else
            (goto _label)))))))

(fn ReleaseGrip
  (params (MotionController :type Grip%20Motion%20Controller%20Component%20Object%20Reference))
  (bind _griparray (Class|GripMotionControllerComponent|GetAllGrips MotionController))
  (for _array_element _griparray
    (Class|GripMotionControllerComponent|DropObjectbyInterface MotionController (.GrippedObject (Utilities|Struct|BreakBPActorGripInformation _array_element)) (.GripID (Utilities|Struct|BreakBPActorGripInformation _array_element)) "0, 0, 0" "0, 0, 0")))

(fn StartUse
  (params (MotionController :type Grip%20Motion%20Controller%20Component%20Object%20Reference))
  (bind _grippedobjectsarray (Class|GripMotionControllerComponent|GetGrippedObjects MotionController))
  (for _array_element _grippedobjectsarray
    (if (Utilities|DoesObjectImplementInterface _array_element "/Script/VRExpansionPlugin.VRGripInterface")
      (Class|VRGripInterface|OnUsed(Message) _array_element))))

(fn AverageSceneComponentTransform
  (params (ComponentA :type Scene%20Component%20Object%20Reference) (ComponentB :type Scene%20Component%20Object%20Reference))
  (return (Math|Transform|MakeTransform (* (+ (Transformation|GetWorldLocation ComponentA) (Transformation|GetWorldLocation ComponentB)) 0.5) (Math|Rotator|Lerp(Rotator) (Transformation|GetWorldRotation ComponentA) (Transformation|GetWorldRotation ComponentB) 0.5 true))))