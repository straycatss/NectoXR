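; Blueprint helper that computes the aiming arc and landing point for teleportation.
; TraceTeleport predicts a projectile path against WorldStatic objects from a start position, direction and velocity, with optional single-frame debug drawing.
; It projects the hit location onto the navigation mesh, returning the arc points, the projected destination and whether that destination is valid.
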(fn TraceTeleport
  (params (Position :type Vector) (Forward :type Vector) (Velocity :type Float%20%28single-precision%29) (Debug :type Boolean))
  (if Debug
    (LocalVariables|SetDebugDrawType "ForOneFrame")
    (else
      (bind _output_get (LocalVariables|SetDebugDrawType "None"))))
  (bind (_outhit _outpathpositions) (Class|GameplayStatics|BlueprintPredictProjectilePathbyObjectType (LocalVariables|Get__WorldContext) Position (* Forward Velocity) true 0.0 (Utilities|Array|MakeArray "ObjectTypeQuery1") false 0 _output_get))
  (return _outpathpositions (.ProjectedLocation (AI|Navigation|ProjectPointtoNavigation (LocalVariables|Get__WorldContext) (.Location (Collision|BreakHitResult _outhit)) 0 0)) (.ReturnValue (AI|Navigation|ProjectPointtoNavigation (LocalVariables|Get__WorldContext) (.Location (Collision|BreakHitResult _outhit)) 0 0))))