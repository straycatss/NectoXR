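; CableJack_A is the grippable jack on the loose end of a cable being drawn between plugs.
; While hovering over a plug, it pairs it with the cable's origin plug to check for an input/output match and updates the cable's ghost status, resetting on exit.
; On release, the server connects the cable to the closest overlapping plug, or destroys the cable if none is found, then destroys the jack.
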(event Collision|EventActorBeginOverlap
  (params (OtherActor :type Actor%20Object%20Reference))
  (bind _owningcable (Variables|Default|GetOwningCable))
  ;[1 1 1] Update the cable depending on what type of object the jack is hovering over
  (bind _hoverplug (Utilities|GetHoveredPlug OtherActor))
  (Utilities|IsValid _hoverplug
    (:Is%20Valid
      (bind _output_get (Variables|Default|SetOverlappingPlug _hoverplug))
      (bind (_inputplug _outputplug) (CallFunction|SortPlugs _output_get (Variables|/Game/Blueprints/ShowtimeEntities/Cable_BP.Cable_BP_C|GetOriginPlug (Variables|Default|GetOwningCable))))
      (if (and (Utilities|IsValid _inputplug) (Utilities|IsValid _outputplug))
        (Default|SetCableGhostStatus _owningcable "NewEnumerator0")
        (else
          (Default|SetCableGhostStatus _owningcable "NewEnumerator1"))))))

(event Collision|EventActorEndOverlap
  (params (OtherActor :type Actor%20Object%20Reference))
  ;[1 1 1] Reset cable visuals
  (bind _hoverplug (Utilities|GetHoveredPlug OtherActor))
  (if (== _hoverplug (Variables|Default|GetOverlappingPlug))
    (Default|SetCableGhostStatus (Variables|Default|GetOwningCable) "NewEnumerator2")))

(event EventOnGrip
  (params (GrippingController :type Grip%20Motion%20Controller%20Component%20Object%20Reference) (GripInformation :type BP%20Actor%20Grip%20Information%20Structure%20%28by%20ref%29))
  (if (Variables|/Game/Blueprints/ShowtimeEntities/Cable_BP.Cable_BP_C|GetbIsDrawing (Variables|Default|GetOwningCable))
    _))

(event EventOnGripRelease
  (params (ReleasingController :type Grip%20Motion%20Controller%20Component%20Object%20Reference) (GripInformation :type BP%20Actor%20Grip%20Information%20Structure%20%28by%20ref%29) (bWasSocketed :type Boolean))
  (bind _owningcable (Variables|Default|GetOwningCable))
  ;[1 1 1] Find nearest valid plug we dropped the cable onto
  (Networking|SwitchHasAuthority
    (:Authority
      (bind _closest (CallFunction|GetClosestGrippableActor (Collision|GetOverlappingActors (Variables|Default|GetStaticMeshComponent) "/Game/Blueprints/ShowtimeEntities/Plug_A_BP.Plug_A_BP_C" :!class /Script/Engine.PrimitiveComponent) (Transformation|GetWorldLocation ReleasingController)))
      (bind _asplug_a_bp (Utilities|Casting|CastToPlug_A_BP _closest)
        (:then
          (Default|ConnectCable _owningcable (Actor|GetComponentbyClass _asplug_a_bp "/Script/ShowtimeRuntime.ShowtimePlug") (Variables|/Game/Blueprints/ShowtimeEntities/Cable_BP.Cable_BP_C|GetOriginPlug _owningcable))
          (Default|SetCableGhostStatus (Variables|Default|GetOwningCable) "NewEnumerator3"))
        (:CastFailed
          ;[1 1 1] Destroy cable if we didn't drop on a valid plug
          (Actor|DestroyActor (Variables|Default|GetOwningCable))))
      (Variables|/Game/Blueprints/ShowtimeEntities/Cable_BP.Cable_BP_C|SetbIsDrawing _owningcable false)
      (Actor|DestroyActor))))

(event EventTickGrip
  (params (GrippingController :type Grip%20Motion%20Controller%20Component%20Object%20Reference) (GripInformation :type BP%20Actor%20Grip%20Information%20Structure%20%28by%20ref%29) (DeltaTime :type Float%20%28single-precision%29))
  (if (Variables|/Game/Blueprints/ShowtimeEntities/Cable_BP.Cable_BP_C|GetbIsDrawing (Variables|Default|GetOwningCable))
    _))

(fn ConstructionScript)