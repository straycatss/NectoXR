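; Actor that draws a teleport aiming arc from its location and forward vector, recording the destination and whether it is valid.
; Every tick, TraceTeleport returns arc points that reshape a spline.
; Spawned pip actors and spline mesh components are added or removed as the point count changes, then repositioned along the arc.
; Pips are destroyed with the actor, and an older mesh-building chain in the event graph is unconnected.
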(event EventDestroyed
  (for _array_element (Variables|Default|GetTeleportPips)
    (Actor|DestroyActor _array_element)))

(event EventTick
  (params (DeltaSeconds :type Float%20%28single-precision%29))
  (CallFunction|UpdateTeleportArc))

(fn ConstructionScript
  (bind _spline (Variables|Default|GetSpline))
  (Spline|ClearSplinePoints _spline true)
  (Spline|AddSplinePoint _spline (Math|Vector|MakeVector 0.0 0.0 0.0) "Local" true))

(fn UpdateTeleportArc
  (bind _defaultsceneroot (Variables|Default|GetDefaultSceneRoot))
  (bind _teleportarcmeshes (Variables|Default|GetTeleportArcMeshes))
  (bind _spline (Variables|Default|GetSpline))
  (bind _teleportpips (Variables|Default|GetTeleportPips))
  (bind _teleportpips_2 (Variables|Default|GetTeleportPips))
  (bind _returnvalue (Utilities|Array|LastIndex _teleportpips))
  (bind _returnvalue_2 (Utilities|Array|LastIndex _teleportarcmeshes))
  (bind _returnvalue_3 (Utilities|Array|Length _teleportpips_2))
  ;[1 1 1] Get arc points
  (bind (_arcpoints _teleportdestination _validdestination) (CallFunction|TraceTeleport (Transformation|GetWorldLocation _defaultsceneroot) (Math|Vector|GetForwardVector _defaultsceneroot) (Variables|Default|GetTeleportArcDistance) false))
  (LocalVariables|SetArcPoints _arcpoints)
  (Variables|Default|SetbIsDestinationValid _validdestination)
  (Variables|Default|SetTeleportDestination _teleportdestination)
  (Spline|SetSplinePoints (Variables|Default|GetSpline) (LocalVariables|GetArcPoints) "World" true)
  (Utilities|FlowControl|Sequence
    (:then_0
      ;[1 1 1] Create/remove pips
      ;;[1 1 1] Create new pips if arc length has changed
      (if (!= (Utilities|Array|Length (LocalVariables|GetArcPoints)) (Utilities|Array|Length (Variables|Default|GetTeleportPips)))
        (if (> _returnvalue_3 (Utilities|Array|Length (LocalVariables|GetArcPoints)))
          ;;[1 1 1] Delta of arc items that need removing
          (for _index (range (- (Utilities|Array|Length (LocalVariables|GetArcPoints)) 1) (- _returnvalue_3 1))
            (Utilities|FlowControl|Sequence
              (:then_0
                ;;[1 1 1] Remove extra pips
                (Actor|DestroyActor (Utilities|Array|Get(acopy) _teleportpips _returnvalue))
                (Utilities|Array|RemoveIndex _teleportpips _returnvalue))
              (:then_1
                ;;[1 1 1] Remove extra spline meshes
                (Components|DestroyComponent (Utilities|Array|Get(acopy) _teleportarcmeshes _returnvalue_2))
                (Utilities|Array|RemoveIndex _teleportarcmeshes _returnvalue_2))))
          (else
            ;;[1 1 1] Delta of arc items that need adding
            (for _index_2 (range (+ _returnvalue_3 1) (+ _returnvalue_3 (- (Utilities|Array|Length (LocalVariables|GetArcPoints)) _returnvalue_3)))
              (Utilities|FlowControl|Sequence
                (:then_0
                  ;;[1 1 1] Create missing pips
                  (bind _returnvalue_4 (Game|SpawnActorfromClass "/Game/Blueprints/Interaction/TeleportPip.TeleportPip_C" (Transformation|GetActorTransform) "Undefined" 0 0))
                  (Utilities|Array|Add (Variables|Default|GetTeleportPips) _returnvalue_4))
                (:then_1
                  ;;[1 1 1] Create missing spline meshes
                  (if (< (- _index_2 1) (Utilities|Array|Length (LocalVariables|GetArcPoints)))
                    (bind _returnvalue_5 (AddComponent|AddSplineMeshComponent true))
                    (Utilities|Array|Add (Variables|Default|GetTeleportArcMeshes) _returnvalue_5)))))))))
    (:then_1
      (Utilities|FlowControl|Sequence
        (:then_0
          ;[1 1 1] Update pip locations
          (for (_array_element _array_index) (Variables|Default|GetTeleportPips)
            (Transformation|SetActorLocation _array_element (Utilities|Array|Get(acopy) (LocalVariables|GetArcPoints) _array_index) false false)))
        (:then_1
          ;[1 1 1] Update spline mesh positions
          (for _index_3 (range 1 (Spline|GetNumberOfSplinePoints (Variables|Default|GetSpline)))
            (SplineMesh|SetStartandEnd (Utilities|Array|Get(acopy) (Variables|Default|GetTeleportArcMeshes) (- _index_3 1)) (.Location (Spline|GetLocationandTangentatSplinePoint _spline (- _index_3 1) "World")) (.Tangent (Spline|GetLocationandTangentatSplinePoint _spline (- _index_3 1) "World")) (.Location (Spline|GetLocationandTangentatSplinePoint _spline _index_3 "World")) (.Tangent (Spline|GetLocationandTangentatSplinePoint _spline _index_3 "World")) true :!class /Script/Engine.SplineMeshComponent)))))))