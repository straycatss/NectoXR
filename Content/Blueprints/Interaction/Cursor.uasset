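; Cursor actor in the Interaction folder that shows a strength value through the size of a cylinder mesh.
; Every tick, UpdateCursor maps CursorStrength from the 0–1 range onto MaxSize down to MinSize, so a stronger value gives a narrower cursor.
; Only the world X and Y scale change; the cylinder keeps its current Z scale.
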(event EventBeginPlay)

(event Collision|EventActorBeginOverlap
  (params (OtherActor :type Actor%20Object%20Reference)))

(event EventTick
  (params (DeltaSeconds :type Float%20%28single-precision%29))
  (CallFunction|UpdateCursor))

(fn ConstructionScript)

(fn UpdateCursor
  (bind _minsize (Variables|Default|GetMinSize))
  (bind _maxsize (Variables|Default|GetMaxSize))
  (bind _cursorstrength (Variables|Default|GetCursorStrength))
  (bind _returnvalue (Math|Float|MapRangeClamped _cursorstrength 0.0 1.0 _maxsize _minsize))
  (Transformation|SetWorldScale3D (Variables|Default|GetCylinder) (Math|Vector|MakeVector _returnvalue _returnvalue (.z (Transformation|GetWorldScale (Variables|Default|GetCylinder))))))