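; VR player character that lets the player grip, release and use objects with left and right motion controllers.
; Grip press searches actors overlapping the collider's owner for a nearby VRGripInterface component or actor, then grips it at its current transform.
; Only the single-collider search is implemented.
; Grip release drops everything that controller holds, and trigger press calls OnUsed on its gripped GrippableStaticMeshActors.
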(event EventBeginPlay
  (bind _leftcolliders (Variables|Default|GetLeftColliders))
  (bind _rightcolliders (Variables|Default|GetRightColliders))
  ;[1 1 1] Make controllers active
  (Utilities|Set|Clear _leftcolliders)
  (Utilities|Set|Clear _rightcolliders)
  (Utilities|Set|Add _leftcolliders (Variables|Default|GetLeftMotionControllerCollision))
  (Utilities|Set|Add _rightcolliders (Variables|Default|GetRightMotionControllerCollision))
  (Rendering|SetVisibility (Variables|Default|GetLeftMotionController) true false)
  (Rendering|SetVisibility (Variables|Default|GetRightMotionController) true false))

(event EventTick
  (params (DeltaSeconds :type Float%20%28single-precision%29)))

(event Input|ActionEvents|InputActionVR_Grip_L
  (params (Key :type Key%20Structure))
  (bind _leftmotioncontroller (Variables|Default|GetLeftMotionController))
  (:Pressed
    ;[1 1 1] Start and release grips
    (CallFunction|StartGrip (Variables|Default|GetLeftColliders) _leftmotioncontroller))
  (:Released
    (CallFunction|ReleaseGrips _leftmotioncontroller)))

(event Input|ActionEvents|InputActionVR_Grip_R
  (params (Key :type Key%20Structure))
  (bind _rightmotioncontroller (Variables|Default|GetRightMotionController))
  (:Pressed
    ;[1 1 1] Start and release grips
    (CallFunction|StartGrip (Variables|Default|GetRightColliders) _rightmotioncontroller))
  (:Released
    (CallFunction|ReleaseGrips _rightmotioncontroller)))

(event Input|ActionEvents|InputActionVR_Trigger_R
  (params (Key :type Key%20Structure))
  (:Pressed
    ;[1 1 1] Use the gripped actor (controller only)
    (CallFunction|StartUse (Variables|Default|GetRightMotionController))))

(event Input|ActionEvents|InputActionVR_Trigger_L
  (params (Key :type Key%20Structure))
  (:Pressed
    ;[1 1 1] Use the gripped actor (controller only)
    (CallFunction|StartUse (Variables|Default|GetLeftMotionController))))

(fn ConstructionScript)

(fn ActorsOverlappingMotionController
  (params (Colliders :type Set%20of%20Scene%20Component%20Object%20References))
  (bind _result (Utilities|Set|ToArray Colliders))
  ;[1 1 1] Only bother with multipler colliders if > 1
  (if (not (> (Utilities|Array|Length _result) 1))
    ;[1 1 1] Check for collision against a single actor
    (LocalVariables|SetCollisionCentroid (Transformation|GetActorLocation (Components|GetOwner (Utilities|Array|Get(acopy) _result (Utilities|Array|LastIndex _result)))))
    (LocalVariables|SetOverlappingActors (Collision|GetOverlappingActors (Components|GetOwner (Utilities|Array|Get(acopy) _result (Utilities|Array|LastIndex _result))) 0 :!class /Script/Engine.Actor))
    (for _array_element (LocalVariables|GetOverlappingActors)
      ;[1 1 1] Grippable component in overlapping actor?
      (if (> (Utilities|Array|Length (Class|Actor|GetComponentsbyInterface _array_element "/Script/VRExpansionPlugin.VRGripInterface")) 0)
        (for _array_element_2 (Class|Actor|GetComponentsbyInterface _array_element "/Script/VRExpansionPlugin.VRGripInterface")
          (Utilities|IsValid (LocalVariables|GetClosestComponent)
            (:Is%20Valid
              (if (< (Math|Vector|VectorLength (- (Transformation|GetActorLocation (Components|GetOwner _array_element_2)) (LocalVariables|GetCollisionCentroid))) (LocalVariables|GetClosestDistance))
                (LocalVariables|SetClosestDistance (Math|Vector|VectorLength (- (Transformation|GetActorLocation (Components|GetOwner _array_element_2)) (LocalVariables|GetCollisionCentroid))) :!label _label)
                (bind _asprimitive_component (Utilities|Casting|CastToPrimitiveComponent _array_element_2))
                (LocalVariables|SetClosestObj _asprimitive_component)))
            (:Is%20Not%20Valid
              (goto _label))))
        (return (LocalVariables|GetClosestObj) (LocalVariables|GetCollisionCentroid))
        (else
          ;[1 1 1] Find closest grippable actor
          (if (Utilities|DoesObjectImplementInterface _array_element "/Script/VRExpansionPlugin.VRGripInterface")
            (Utilities|IsValid (LocalVariables|GetClosestObj)
              (:Is%20Valid
                (if (< (Math|Vector|VectorLength (- (Transformation|GetActorLocation _array_element) (LocalVariables|GetCollisionCentroid))) (LocalVariables|GetClosestDistance))
                  (LocalVariables|SetClosestDistance (Math|Vector|VectorLength (- (Transformation|GetActorLocation _array_element) (LocalVariables|GetCollisionCentroid))) :!label _label_2)
                  (LocalVariables|SetClosestObj _array_element)))
              (:Is%20Not%20Valid
                (goto _label_2)))))))
    (return (LocalVariables|GetClosestObj) (LocalVariables|GetCollisionCentroid))))

(fn ReleaseGrips
  (params (MotionController :type Grip%20Motion%20Controller%20Component%20Object%20Reference))
  (bind _griparray (Class|GripMotionControllerComponent|GetAllGrips MotionController))
  (for _array_element _griparray
    (Class|GripMotionControllerComponent|DropObjectbyInterface MotionController (Variables|Default|GetGrippedActor) (.GripID (Utilities|Struct|BreakBPActorGripInformation _array_element)) "0, 0, 0" "0, 0, 0")))

(fn StartGrip
  (params (Colliders :type Set%20of%20Scene%20Component%20Object%20References) (MotionController :type Grip%20Motion%20Controller%20Component%20Object%20Reference))
  (bind _closestobject (CallFunction|ActorsOverlappingMotionController Colliders))
  ;[1 1 1] Grip a component
  (Utilities|IsValid _closestobject
    (:Is%20Valid
      (bind _asprimitive_component (Utilities|Casting|CastToPrimitiveComponent _closestobject)
        (:then
          (Class|GripMotionControllerComponent|GripObjectbyInterface MotionController _asprimitive_component (Transformation|GetWorldTransform _asprimitive_component) false "None" "None" false))
        (:CastFailed
          ;[1 1 1] Grip an actor
          (bind _asactor (Utilities|Casting|CastToActor _closestobject))
          (Class|GripMotionControllerComponent|GripObjectbyInterface MotionController _asactor (Transformation|GetWorldTransform (Variables|/Script/Engine.Actor|GetRootComponent _asactor)) false "None" "None" false))))))

(fn StartUse
  (params (MotionController :type Grip%20Motion%20Controller%20Component%20Object%20Reference))
  (bind _grippedactorarray (Class|GripMotionControllerComponent|GetGrippedActors MotionController))
  (for _array_element _grippedactorarray
    (bind _asgrippable_static_mesh_actor (Utilities|Casting|CastToGrippableStaticMeshActor _array_element))
    (Class|GrippableStaticMeshActor|OnUsed _asgrippable_static_mesh_actor)))