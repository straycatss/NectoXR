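; GrippingFUnctions provides a helper that picks which overlapping actor is the closest candidate for a VR grip.
; GetClosestGrippableActor loops over the supplied actors, keeping only those that implement VRGripInterface.
; It compares each actor's location to the collision point and returns the nearest, measuring to actor origins rather than component surfaces.
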(fn GetClosestGrippableActor
  (params (OverlappingActors :type Array%20of%20Actor%20Object%20References) (CollisionPoint :type Vector))
  ;[1 1 1] Find closest grippable actor
  (for _array_element OverlappingActors
    (if (Utilities|DoesObjectImplementInterface _array_element "/Script/VRExpansionPlugin.VRGripInterface")
      (Utilities|IsValid (LocalVariables|GetClosestActor)
        (:Is%20Valid
          (if (< (Math|Vector|VectorLength (- (Transformation|GetActorLocation _array_element) CollisionPoint)) (LocalVariables|GetClosestDistance))
            (LocalVariables|SetClosestDistance (Math|Vector|VectorLength (- (Transformation|GetActorLocation _array_element) CollisionPoint)) :!label _label)
            (bind _output_get (LocalVariables|SetClosestActor _array_element))))
        (:Is%20Not%20Valid
          (goto _label)))))
  (return _output_get))