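; Grippable beacon actor that represents a named server, which its owning client joins when the beacon is used.
; The authority hands ownership to the gripping controller and spawns an attached camera-facing label, with RepNotifies keeping its name text updated.
; Client connected, disconnected and server-lost events, filtered by server name, drive timelines on a dynamic material's Connected and Opacity parameters to show status and fade the beacon.
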(event Custom|OnBeaconActivated
  ;[1 1 1] Use beacon to join
  (Class|ShowtimeClient|JoinServerbyName (Variables|Default|GetOwningClient) (Variables|Default|GetServerName)))

(event Custom|OnBeaconConnected
  (params (Client :type Showtime%20Client%20Object%20Reference) (ServerAddress :type Server%20Address%20Structure))
  ;[1 1 1] Fade on connected/disconnected
  (if (Utilities|Enum|Equal(Enum) (.name ServerAddress) (Variables|Default|GetServerName))
    (bind _connectedtransitionval (Timeline|connected_transition PlayFromStart)
      (:Update
        (Rendering|Material|SetScalarParameterValue (Variables|Default|GetBeaconMaterial) "Connected" _connectedtransitionval :!class /Script/Engine.MaterialInstanceDynamic)))))

(event Custom|OnBeaconDisconnected
  (params (Client :type Showtime%20Client%20Object%20Reference) (ServerAddress :type Server%20Address%20Structure))
  ;[1 1 1] Fade on connected/disconnected
  (if (Utilities|Enum|Equal(Enum) (.name ServerAddress) (Variables|Default|GetServerName))
    (bind _connectedtransitionval (Timeline|connected_transition ReverseFromEnd)
      (:Update
        (Rendering|Material|SetScalarParameterValue (Variables|Default|GetBeaconMaterial) "Connected" _connectedtransitionval :!class /Script/Engine.MaterialInstanceDynamic)))))

(event Custom|OnBeaconLost
  (params (Client :type Showtime%20Client%20Object%20Reference) (ServerAddress :type Server%20Address%20Structure))
  ;[1 1 1] Fade on connected/disconnected
  (if (Utilities|Enum|Equal(Enum) (.name ServerAddress) (Variables|Default|GetServerName))
    (bind (_direction _connectedtransitionval) (Timeline|fade_transition ReverseFromEnd)
      (:Update
        (Rendering|Material|SetScalarParameterValue (Variables|Default|GetBeaconMaterial) "Opacity" _connectedtransitionval :!class /Script/Engine.MaterialInstanceDynamic))
      (:Finished
        (switch Utilities|FlowControl|Switch|SwitchonETimelineDirection _direction
          (:Backward
            (Networking|SwitchHasAuthority
              (:Authority
                (Actor|DestroyActor)))))))))

(event EventBeginPlay
  (Networking|SwitchHasAuthority
    (:Authority
      ;[1 1 1] Create and set up replicated components
      (CallFunction|CreateCameraFacingLabel)
      (Utilities|FlowControl|Delay 1.0)
      (Default|SetCamera (Variables|Default|GetLabel)))
    (:Remote
      ;[1 1 1] Fade on connected/disconnected
      (bind (_direction _connectedtransitionval) (Timeline|fade_transition PlayFromStart)
        (:Update
          (Rendering|Material|SetScalarParameterValue (Variables|Default|GetBeaconMaterial) "Opacity" _connectedtransitionval :!class /Script/Engine.MaterialInstanceDynamic))
        (:Finished
          (switch Utilities|FlowControl|Switch|SwitchonETimelineDirection _direction
            (:Backward
              (Networking|SwitchHasAuthority
                (:Authority
                  (Actor|DestroyActor))))))))))

(event EventOnGrip
  (params (GrippingController :type Grip%20Motion%20Controller%20Component%20Object%20Reference) (GripInformation :type BP%20Actor%20Grip%20Information%20Structure%20%28by%20ref%29))
  ;[1 1 1] On grip change ownership to playercontroller
  (Networking|SwitchHasAuthority
    (:Authority
      (Actor|SetOwner (Components|GetOwner GrippingController)))))

(event EventOnUsed
  ;[1 1 1] Use beacon to join
  (CallFunction|OnBeaconActivated))

(event EventOnGripRelease
  (params (ReleasingController :type Grip%20Motion%20Controller%20Component%20Object%20Reference) (GripInformation :type BP%20Actor%20Grip%20Information%20Structure%20%28by%20ref%29) (bWasSocketed :type Boolean))
  ;[1 1 1] On release restore ownership to server
  (Networking|SwitchHasAuthority
    (:Authority
      (Actor|SetOwner (Components|GetOwner)))))

(fn ConstructionScript
  (bind _returnvalue (Rendering|Material|CreateDynamicMaterialInstance (Variables|Default|GetStaticMeshComponent) 0 "/Game/Materials/ServerBeacon_Mat.ServerBeacon_Mat" "None" :!class /Script/Engine.PrimitiveComponent))
  (Variables|Default|SetBeaconMaterial _returnvalue))

(fn SetOwningClient
  (params (Client :type Showtime%20Client%20Object%20Reference%20%28by%20ref%29))
  (bind _output_get (Variables|Default|SetOwningClient Client))
  (EventDispatchers|BindEventtoOnConnectedtoServer _output_get (EventDispatchers|CreateEvent :!event Custom|OnBeaconConnected))
  (EventDispatchers|BindEventtoOnDisconnectedfromServer _output_get (EventDispatchers|CreateEvent :!event Custom|OnBeaconDisconnected))
  (EventDispatchers|BindEventtoOnServerLost _output_get (EventDispatchers|CreateEvent :!event Custom|OnBeaconLost)))

(fn CreateCameraFacingLabel
  (Networking|SwitchHasAuthority
    (:Authority
      (bind _returnvalue (Game|SpawnActorfromClass "/Game/Blueprints/CameraFacingTextActor_BP.CameraFacingTextActor_BP_C" (Math|Transform|MakeTransform "0, 0, 0") "Undefined" self (Variables|Default|GetServerName) 0))
      (Transformation|AttachComponentToComponent _returnvalue (Variables|Default|GetBox) "None" "KeepRelative" "KeepRelative" "KeepRelative" true)
      (Variables|Default|SetLabel _returnvalue))))

(fn OnRepServerName
  (bind _self self)
  (bind _label (Variables|Default|GetLabel _self))
  (Utilities|IsValid _label
    (:Is%20Valid
      (Rendering|Components|TextRender|SetText (Variables|/Game/Blueprints/CameraFacingTextActor_BP.CameraFacingTextActor_BP_C|GetText _label) (Utilities|Text|ToText(String) (Variables|Default|GetServerName))))))

(fn OnRepLabel
  (Rendering|Components|TextRender|SetText (Variables|/Game/Blueprints/CameraFacingTextActor_BP.CameraFacingTextActor_BP_C|GetText (Variables|Default|GetLabel)) (Utilities|Text|ToText(String) (Variables|Default|GetServerName))))