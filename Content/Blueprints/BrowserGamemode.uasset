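; BrowserGamemode is a game mode for a lobby that shows discovered Showtime graph servers as beacon actors.
; On BeginPlay it initializes the Showtime client, suffixing the client name on the server, and it leaves on EndPlay.
; While unconnected, discoveries spawn ServerBeacon_BP at the "lobby_start" player start and map it by name.
; Server loss only removes the map entry, and auto-join logic is left unwired.
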(event OnServerDiscovered(ShowtimeClient)
  (params (Client :type Showtime%20Client%20Object%20Reference) (ServerAddress :type Server%20Address%20Structure))
  ;[1 1 1] Server discovery
  (bind _returnvalue (Class|ShowtimeClient|IsConnected Client))
  (if (not _returnvalue)
    ;[1 1 1] Spawn beacon
    (bind _returnvalue_2 (Game|SpawnActorfromClass "/Game/Blueprints/ServerBeacon_BP.ServerBeacon_BP_C" (Transformation|GetActorTransform (Class|GameModeBase|FindPlayerStart 0 "lobby_start")) "Undefined" 0 (.name ServerAddress) 0))
    (Default|SetOwningClient _returnvalue_2 Client)
    (Utilities|Map|Add (Variables|Default|Getservers) (.name ServerAddress) _returnvalue_2)))

(event OnConnectedtoServer(ShowtimeClient)
  (params (Client :type Showtime%20Client%20Object%20Reference) (ServerAddress :type Server%20Address%20Structure))
  (Variables|Default|Setconnected true)
  (Development|PrintString (Utilities|String|Append "Connected to graph server " (.name (Utilities|Struct|BreakServerAddress ServerAddress)))))

(event OnServerLost(ShowtimeClient)
  (params (Client :type Showtime%20Client%20Object%20Reference) (ServerAddress :type Server%20Address%20Structure))
  ;[1 1 1] Server discovery
  (if (Networking|IsServer)
    (Utilities|Map|Remove (Variables|Default|Getservers) (.name ServerAddress))))

(event EventBeginPlay
  (CallFunction|InitClient))

(event EventTick
  (params (DeltaSeconds :type Float%20%28single-precision%29)))

(event EventEndPlay
  (params (EndPlayReason :type EEndPlayReason%20Enum :default "Destroyed"))
  (Class|ShowtimeClient|LeaveServer (Variables|Default|GetShowtimeClient)))

(fn ConstructionScript)

(fn InitClient
  (bind _showtimeclient (Variables|Default|GetShowtimeClient))
  ;[1 1 1] Init Showtime client
  (if (Networking|IsServer)
    (Variables|/Script/ShowtimeRuntime.ShowtimeClient|SetClientName _showtimeclient (Utilities|String|Append (Variables|/Script/ShowtimeRuntime.ShowtimeClient|GetClientName _showtimeclient) "_serv")))
  (Class|ShowtimeClient|Init _showtimeclient)
  (return))